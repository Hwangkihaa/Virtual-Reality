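; BP_Bullet is a projectile Actor that destroys any BP_DummyTarget it hits.
; Each Tick it moves along its forward vector with a swept world offset scaled by Speed and delta time, without a movement component.
; A Sphere hit prints the other actor's name, destroys it if it is a dummy target, then always destroys the bullet.
; A timer started on BeginPlay also destroys the bullet after a short lifetime.
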(event OnComponentHit(Sphere)
  (params (HitComponent :type Primitive%20Component%20Object%20Reference) (OtherActor :type Actor%20Object%20Reference) (OtherComp :type Primitive%20Component%20Object%20Reference) (NormalImpulse :type Vector :default "0, 0, 0") (Hit :type Hit%20Result%20Structure%20%28by%20ref%29))
  (Development|PrintString (Utilities|GetDisplayName OtherActor))
  (Utilities|FlowControl|Sequence
    (:then_0
      (bind _asbp_dummy_target (Utilities|Casting|CastToBP_DummyTarget OtherActor))
      (Actor|DestroyActor _asbp_dummy_target))
    (:then_1
      (Actor|DestroyActor))))

(event Custom|TimeTiDestroy
  (Development|PrintString "Destroy Bullet")
  (Actor|DestroyActor))

(event EventBeginPlay
  (Utilities|Time|SetTimerbyEvent (delegate Custom|TimeTiDestroy) 2.0))

(event Collision|EventActorBeginOverlap
  (params (OtherActor :type Actor%20Object%20Reference)))

(event EventTick
  (params (DeltaSeconds :type Float%20%28single-precision%29))
  (CallFunction|MoveForward DeltaSeconds))

(fn ConstructionScript)

(fn MoveForward
  (params (TimeDelta :type Float%20%28double-precision%29))
  (Transformation|AddActorWorldOffset (* (* TimeDelta (Variables|Default|GetSpeed)) (Math|Vector|GetForwardVector (Transformation|GetActorRotation))) true))