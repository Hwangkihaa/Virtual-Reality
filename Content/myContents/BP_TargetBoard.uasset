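; BP_TargetBoard is a target board that pivots between standing and lying down.
; When a BP_myCharacter overlaps the UpSwitch actor, it calls EventStandUp; EventDown has no caller in this file.
; Two timelines drive the board's relative pitch.
; A status gate accepts each event only from the opposite end state, holding an intermediate Ready state during motion to block retriggers.
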(event OnActorBeginOverlap(upSwitch)
  (params (OverlappedActor :type Actor%20Object%20Reference) (OtherActor :type Actor%20Object%20Reference))
  (Utilities|Casting|CastToBP_myCharacter OtherActor)
  (CallFunction|EventStandUp))

(event Custom|EventStandUp
  (switch Utilities|FlowControl|Switch|Switchonenum_TargetState (Variables|Default|GetCurrentStatus)
    (:NewEnumerator2
      (Variables|Default|SetCurrentStatus "NewEnumerator0")
      (bind _target_stand (Timeline|Timeline_up PlayFromStart)
        (:Update
          (Transformation|SetRelativeRotation (Variables|Default|GetTargetBoard) (Math|Rotator|MakeRotator 0.0 _target_stand 0.0) false false))
        (:Finished
          (Variables|Default|SetCurrentStatus "NewEnumerator1"))))))

(event Custom|EventDown
  (switch Utilities|FlowControl|Switch|Switchonenum_TargetState (Variables|Default|GetCurrentStatus)
    (:NewEnumerator1
      (Variables|Default|SetCurrentStatus "NewEnumerator0")
      (bind _target_stand (Timeline|Timeline_down PlayFromStart)
        (:Update
          (Transformation|SetRelativeRotation (Variables|Default|GetTargetBoard) (Math|Rotator|MakeRotator 0.0 _target_stand 0.0) false false))
        (:Finished
          (Variables|Default|SetCurrentStatus "NewEnumerator2"))))))

(event EventBeginPlay)

(event Collision|EventActorBeginOverlap
  (params (OtherActor :type Actor%20Object%20Reference)))

(event EventTick
  (params (DeltaSeconds :type Float%20%28single-precision%29)))

(fn ConstructionScript)