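; Player character Blueprint with gun firing, ammo, reload and a game countdown that quits when time runs out.
; BeginPlay adds the Enhanced Input mapping context; IA_Extra spawns BP_Bullet at Frontgun while Ammo remains.
; Ammo decrements on a separate right-mouse key event, and R refills it to MaxAmmo, with printed feedback.
; Tick uses a Delay to step Minutes and Seconds down about once per second.
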(event Input|EnhancedActionEvents|EnhancedInputActionIA_Extra
  (params (ActionValue :type Boolean) (ElapsedSeconds :type Float%20%28double-precision%29) (TriggeredSeconds :type Float%20%28double-precision%29) (InputAction :type Input%20Action%20Object%20Reference :default "/Game/myContents/IA_Extra.IA_Extra"))
  (if (> (Variables|Default|GetAmmo) 0)
    (Development|PrintString "Fired")
    (Game|SpawnActorfromClass "/Game/myContents/BP_Bullet.BP_Bullet_C" (Transformation|GetWorldTransform (Variables|Default|Getfrontgun)) "Undefined" "MultiplyWithRoot" 0 0)
    (else
      (Development|PrintString "총알 없음 - 발사 불가 !"))))

(event EventBeginPlay
  (|CallParentFunction)
  (Development|PrintString "BeginMyChracter")
  (bind _asplayer_controller (Utilities|Casting|CastToPlayerController (Pawn|GetController)))
  (Input|AddMappingContext (PlayerController|LocalPlayerSubsystems|GetEnhancedInputLocalPlayerSubsystem _asplayer_controller) "/Game/myContents/IMC_myInputContext.IMC_myInputContext" -1 "(bIgnoreAllPressedKeysUntilRelease=True,bForceImmediately=False,bNotifyUserSettings=False)"))

(event EventTick
  (params (DeltaSeconds :type Float%20%28single-precision%29))
  (Utilities|FlowControl|Delay 1.0)
  (if (== (Variables|Default|GetSeconds) 0)
    (if (== (Variables|Default|GetMinutes) 0)
      (Development|PrintString "게임 종료!")
      (Utilities|FlowControl|Delay 5.0)
      (Game|QuitGame 0 "Quit" false)
      (else
        (Variables|Default|SetSeconds 59)
        (Variables|Default|SetMinutes (- (Variables|Default|GetMinutes) 1))))
    (else
      (Variables|Default|SetSeconds (- (Variables|Default|GetSeconds) 1)))))

(event Input|MouseEvents|RightMouseButton
  (params (Key :type Key%20Structure))
  (bind _ammo (Variables|Default|GetAmmo))
  (:Pressed
    (if (> _ammo 0)
      (bind _result (Math|Integer|DecrementInt _ammo)
        (:%20%20
          (Development|PrintText (Utilities|Text|FormatText "{0}" _result)))))))

(event Input|KeyboardEvents|R
  (params (Key :type Key%20Structure))
  (bind _max_ammo (Variables|Default|GetMax%20Ammo))
  (:Pressed
    (if (!= (Variables|Default|GetAmmo) _max_ammo)
      (Development|PrintString "재장전!")
      (bind _output_get (Variables|Default|SetAmmo _max_ammo))
      (Development|PrintText (Utilities|Text|FormatText "{0}" _output_get))
      (else
        (Development|PrintText "총알 가득 참!")))))

(fn ConstructionScript
  (|CallParentFunction))